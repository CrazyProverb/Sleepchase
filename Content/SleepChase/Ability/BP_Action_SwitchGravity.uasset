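; Gameplay action that switches a character's gravity direction while it is active.
; On start and on stop, it casts the instigator to CharacterBase, calls the parent action, then sets the CharacterMovement gravity direction to a start or end target respectively.
; Each transition prints a debug string, and nothing runs if the cast fails.
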(event `self.StartAction`
  (params (Instigator :type "Actor Object Reference"))
  (bind _ascharacter_base (cast `CharacterBase` Instigator))
  (`parent.StartAction` Instigator)
  (`CharacterMovementComponent.SetGravityDirection` (`Character.CharacterMovement` _ascharacter_base) (`self.Target Gravity Start`))
  (`KismetSystemLibrary.PrintString` "start'"))

(event `self.StopAction`
  (params (Instigator :type "Actor Object Reference"))
  (bind _ascharacter_base (cast `CharacterBase` Instigator))
  (`parent.StopAction` Instigator)
  (`CharacterMovementComponent.SetGravityDirection` (`Character.CharacterMovement` _ascharacter_base) (`self.Target Gravity End`))
  (`KismetSystemLibrary.PrintString` "stop"))